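; BP_RangedSlime is a ranged slime enemy Blueprint that adds procedural idle and attack motion to its mesh.
; On BeginPlay it runs the parent logic, caches the mesh's world scale, and plays a timeline that multiplies that scale by an Idle curve.
; OnAttack restarts a second timeline whose Attack curve is added to the mesh's local X offset each update, so the movement accumulates.
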(event EventBeginPlay
  (|CallParentFunction)
  (Variables|Default|SetInitialScale (Transformation|GetWorldScale (Variables|Character|GetMesh)))
  (bind _idle (Timeline|Timeline Play)
    (:Update
      (Transformation|SetWorldScale3D (Variables|Character|GetMesh) (* _idle (Variables|Default|GetInitialScale))))))

(event Collision|EventActorBeginOverlap
  (params (OtherActor :type Actor%20Object%20Reference))
  (|CallParentFunction OtherActor) ; This node is disabled and will not be called.\nDrag off pins to build functionality.
)

(event EventTick
  (params (DeltaSeconds :type Float%20%28single-precision%29))
  (|CallParentFunction DeltaSeconds) ; This node is disabled and will not be called.\nDrag off pins to build functionality.
)

(event EventOnAttack
  (bind _attack (Timeline|Timeline_0 PlayFromStart)
    (:Update
      (Transformation|AddLocalOffset (Variables|Character|GetMesh) (Math|Vector|MakeVector _attack 0.0 0.0) false false))))

(fn ConstructionScript
  (|CallParentFunction))