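; BP_MeleeSlime is a melee slime enemy Blueprint that animates its mesh procedurally with timelines.
; On BeginPlay it caches the mesh's world scale and plays an Idle timeline that scales the mesh relative to that value.
; OnAttack restarts an Attack timeline, adding its curve value as a local X offset on every update, so movement accumulates rather than setting an absolute position.
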(event EventBeginPlay
  (Variables|Default|SetInitialScale (Transformation|GetWorldScale (Variables|Character|GetMesh)))
  (bind _idle (Timeline|Idle Play)
    (:Update
      (Transformation|SetWorldScale3D (Variables|Character|GetMesh) (* _idle (Variables|Default|GetInitialScale))))))

(event EventOnAttack
  (bind _attack (Timeline|Attack PlayFromStart)
    (:Update
      (Transformation|AddLocalOffset (Variables|Character|GetMesh) (Math|Vector|MakeVector _attack 0.0 0.0) false false))))

(fn ConstructionScript
  (|CallParentFunction))