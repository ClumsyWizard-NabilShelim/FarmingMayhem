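; BP_PlayerCharacter is the player character Blueprint, containing a timeline-driven idle scale animation on its Mesh.
; BeginPlay caches the mesh's world scale, then plays the IdleScale timeline, which multiplies that cached scale by its Idle track on each update.
; An IdlePosition timeline that would add local offsets to the mesh is present but never triggered, and the construction script is empty.
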(event EventBeginPlay
  (Variables|Default|SetInitialScale (Transformation|GetWorldScale (Variables|Character|GetMesh)))
  (bind _idle (Timeline|IdleScale Play)
    (:Update
      (Transformation|SetWorldScale3D (Variables|Character|GetMesh) (* _idle (Variables|Default|GetInitialScale))))))

(fn ConstructionScript)