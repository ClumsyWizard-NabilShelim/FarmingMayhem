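; BP_BaseResource is a base foraging resource that animates its mesh while idle and when damaged.
; On BeginPlay it caches the mesh's world scale, then an Idle timeline multiplies that scale.
; OnDamage zeroes the mesh's relative location and restarts a Jerk timeline, which adds its value as a local offset each update, so offsets accumulate during playback.
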(event EventBeginPlay
  (Variables|Default|SetInitialScale (Transformation|GetWorldScale (Variables|Character|GetMesh)))
  (bind _idle (Timeline|Idle Play)
    (:Update
      (Transformation|SetWorldScale3D (Variables|Character|GetMesh) (* (Variables|Default|GetInitialScale) _idle)))))

(event EventOnDamage
  (Transformation|SetRelativeLocation (Variables|Character|GetMesh) "0, 0, 0" false false)
  (bind _jerk (Timeline|Jerk PlayFromStart)
    (:Update
      (Transformation|AddLocalOffset (Variables|Character|GetMesh) _jerk false false))))

(fn ConstructionScript)